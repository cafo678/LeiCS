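; Player controller Blueprint that turns Enhanced Input move and look actions into player movement and camera rotation.
; Move input feeds MoveRight and MoveForward, look input adds yaw and pitch, and a flag tracks whether movement input is released.
; Releasing movement also ends sprint through EndActionChecked, which stops an action by gameplay tag on the player pawn's action component only if that tag is active.
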(event Input|EnhancedActionEvents|EnhancedInputActionIA_Move
  (params (ActionValue :type Vector%202D%20Structure) (ElapsedSeconds :type Float%20%28double-precision%29) (TriggeredSeconds :type Float%20%28double-precision%29) (InputAction :type Input%20Action%20Object%20Reference :default "/Game/Input/IA_Move.IA_Move"))
  ;[1 1 1] Movement
  (:Triggered
    (Class|LeiPlayerController|MoveRight (.x ActionValue))
    (Class|LeiPlayerController|MoveForward (.y ActionValue))
    (Variables|Default|SetHasUserReleasedMovementInput false))
  (:Completed
    (Variables|Default|SetHasUserReleasedMovementInput true)
    (CallFunction|EndActionChecked "(TagName=\"Action.Sprint\")")))

(event Input|EnhancedActionEvents|EnhancedInputActionIA_Look
  (params (ActionValue :type Vector%202D%20Structure) (ElapsedSeconds :type Float%20%28double-precision%29) (TriggeredSeconds :type Float%20%28double-precision%29) (InputAction :type Input%20Action%20Object%20Reference :default "/Game/Input/IA_Look.IA_Look"))
  ;[1 1 1] Camera
  (:Triggered
    (Class|PlayerController|AddYawInput (.x ActionValue))
    (Class|PlayerController|AddPitchInput (.y ActionValue))))

(fn ConstructionScript)

(fn EndActionChecked
  (params (ActionTagID :type Gameplay%20Tag%20Structure))
  (bind _returnvalue (Class|LeiActionComponentInterface|GetActionComponent(Message) (Game|Player|GetPlayerPawn 0)))
  (if (GameplayTags|HasTag (Variables|/Script/LeiCS.LeiActionComponent|GetActiveGameplayTags _returnvalue) ActionTagID true)
    (Class|LeiActionComponent|StopActionbyTagID _returnvalue self ActionTagID)))