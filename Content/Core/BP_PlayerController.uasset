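; Player controller for opponent-based combat that routes movement and right-stick input and manages the HUD, locked-enemy attributes and debug menu.
; Releasing movement stops Sprint through the pawn's action component.
; Entering combat watches opponent Poise to show a deathblow prompt at zero; pressing the right stick triggers Deathblow on a Staggered opponent.
; Overridden parent combat events forward to BP handlers, which re-check gameplay-state input when actions stop.
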(event Input|EnhancedActionEvents|EnhancedInputActionIA_Move
  (params (ActionValue :type Vector%202D%20Structure) (ElapsedSeconds :type Float%20%28double-precision%29) (TriggeredSeconds :type Float%20%28double-precision%29) (InputAction :type Input%20Action%20Object%20Reference :default "/Game/Input/IA_Move.IA_Move"))
  ;[1 1 1] Movement
  (:Triggered
    (Class|LeiPlayerController|MoveRight (.x ActionValue))
    (Class|LeiPlayerController|MoveForward (.y ActionValue))
    (Variables|Default|SetHasUserReleasedMovementInput false))
  (:Completed
    (Variables|Default|SetHasUserReleasedMovementInput true)
    (bind _returnvalue (Class|LeiActionComponentInterface|GetActionComponent(Message) (Game|Player|GetPlayerPawn 0)))
    (Class|LeiActionComponent|StopActionbyTagID _returnvalue self "(TagName=\"Action.Sprint\")" "None")))

(event Input|EnhancedActionEvents|EnhancedInputActionIA_RightStick
  (params (ActionValue :type Vector%202D%20Structure) (ElapsedSeconds :type Float%20%28double-precision%29) (TriggeredSeconds :type Float%20%28double-precision%29) (InputAction :type Input%20Action%20Object%20Reference :default "/Game/Input/IA_RightStick.IA_RightStick"))
  ;[1 1 1] Right Stick (Camera, Actions)
  (:Triggered
    (Class|LeiPlayerController|HandleRightStick (.x ActionValue) (.y ActionValue)))
  (:Completed
    (Class|LeiPlayerController|OnRightStickReleased)))

(event Input|EnhancedActionEvents|EnhancedInputActionIA_RightStickPressed
  (params (ActionValue :type Boolean) (ElapsedSeconds :type Float%20%28double-precision%29) (TriggeredSeconds :type Float%20%28double-precision%29) (InputAction :type Input%20Action%20Object%20Reference :default "/Game/Input/IA_RightStickPressed.IA_RightStickPressed"))
  ;[1 1 1] Right Stick (Camera, Actions)
  (:Started
    (Input|HandleRightStickPressed)))

(event EventOnOpponentSet
  (params (NewOpponent :type Actor%20Object%20Reference))
  ;[1 1 1] Enemy Attribute Widget
  (|CallParentFunction NewOpponent)
  (Variables|Default|GetEnemyAttributeWidget
    (:then
      (Utilities|IsValid NewOpponent
        (:Is%20Not%20Valid
          (Widget|RemovefromParent (Variables|Default|GetEnemyAttributeWidget))
          (Variables|Default|SetEnemyAttributeWidget 0))))
    (:else
      (Utilities|IsValid NewOpponent
        (:Is%20Valid
          (bind _returnvalue (UserInterface|CreateWidget "/Game/UI/WBP_LockedEnemyAttributes.WBP_LockedEnemyAttributes_C" self NewOpponent))
          (bind _output_get (Variables|Default|SetEnemyAttributeWidget _returnvalue))
          (UserInterface|Viewport|AddtoViewport _output_get 0))))))

(event EventOnPawnActionStopped
  (params (ControlledPawn :type Actor%20Object%20Reference) (ActionTagID :type Gameplay%20Tag%20Structure) (ActionDirectionTag :type Gameplay%20Tag%20Structure) (bIsDirectional :type Boolean))
  (|CallParentFunction ControlledPawn ActionTagID ActionDirectionTag bIsDirectional)
  (Delegates|OnPawnActionStoppedBP ActionTagID))

(event EventBeginPlay
  ;[1 1 1] Add UI
  (bind _returnvalue (UserInterface|CreateWidget "/Game/UI/WBP_MainHUD.WBP_MainHUD_C" self))
  (bind _output_get (Variables|Default|SetMainHUDWidget _returnvalue))
  (UserInterface|Viewport|AddtoViewport _output_get 0))

(event EventOnOpponentActionStopped
  (params (OpponentActor :type Actor%20Object%20Reference) (ActionTagID :type Gameplay%20Tag%20Structure) (ActionDirectionTag :type Gameplay%20Tag%20Structure) (bIsDirectional :type Boolean))
  (|CallParentFunction OpponentActor ActionTagID ActionDirectionTag bIsDirectional)
  (Delegates|OnOpponentActionStoppedBP ActionTagID))

(event EventOnPawnCombatSceneEntered
  (params (OpponentActor :type Actor%20Object%20Reference))
  (|CallParentFunction OpponentActor)
  (Delegates|OnPawnCombatSceneEnteredBP OpponentActor))

(event Input|GamepadEvents|GamepadSpecialRight
  (params (Key :type Key%20Structure))
  ;[1 1 1] Debug Menu
  (:Pressed
    (bind _debugmenuwidget (Variables|Default|GetDebugMenuWidget)
      (:then
        (Widget|RemovefromParent _debugmenuwidget)
        (Variables|Default|SetDebugMenuWidget 0)
        (Input|SetInputModeGameOnly self false))
      (:else
        (bind _returnvalue (UserInterface|CreateWidget "/Game/UI/WBP_DebugMenu.WBP_DebugMenu_C" self))
        (bind _output_get (Variables|Default|SetDebugMenuWidget _returnvalue))
        (UserInterface|Viewport|AddtoViewport _output_get 0)))))

(fn ConstructionScript)

(fn HandleRightStickPressed
  (bind _returnvalue (Class|LeiActionComponentInterface|GetActionComponent(Message) (Pawn|GetControlledPawn)))
  (bind _output_get (LocalVariables|SetPawnActionComponent _returnvalue))
  (bind _returnvalue_2 (Class|LeiActionComponentInterface|GetActionComponent(Message) (Variables|/Script/LeiCS.LeiActionComponent|GetOpponent _output_get)))
  (if (GameplayTags|HasTag (Variables|/Script/LeiCS.LeiActionComponent|GetActiveGameplayTags _returnvalue_2) "(TagName=\"Status.Staggered\")" true)
    (Class|LeiActionComponent|StartActionbyTagID (LocalVariables|GetPawnActionComponent) self "(TagName=\"Action.Deathblow\")")
    (Widget|RemovefromParent (Variables|Default|GetDeathblowWidget))
    (Variables|Default|SetDeathblowWidget 0)))

(fn OnOpponentActionStartedBP
  (params (ActionTagID :type Gameplay%20Tag%20Structure) (ActionDirectionTag :type Gameplay%20Tag%20Structure)))

(fn OnPawnActionStoppedBP
  (params (ActionTagID :type Gameplay%20Tag%20Structure))
  (|SwitchGameplayTag ActionTagID
    (:Action.Deathblow
      (Class|LeiPlayerController|CheckGameplayStateInput))))

(fn OnOpponentActionStoppedBP
  (params (ActionTag :type Gameplay%20Tag%20Structure))
  (|SwitchGameplayTag ActionTag
    (:Action.Deathblow
      (Class|LeiPlayerController|CheckGameplayStateInput))))

(fn OnPawnCombatSceneEnteredBP
  (params (Opponent :type Object%20Object%20Reference))
  (bind _returnvalue (Class|LeiActionComponentInterface|GetActionComponent(Message) Opponent))
  (Class|LeiAttributeSet|AddAttributeChangedDelegate (Variables|/Script/LeiCS.LeiActionComponent|GetAttributeSet _returnvalue) "(TagName=\"Attribute.Poise\")" (EventDispatchers|CreateEvent :!event OnOpponentPoiseChanged)))

(fn OnOpponentPoiseChanged
  (params (Value :type Float%20%28single-precision%29) (MaxValue :type Float%20%28single-precision%29) (MinValue :type Float%20%28single-precision%29))
  (if (<= Value 0.0)
    (bind _returnvalue (Class|LeiActionComponentInterface|GetActionComponent(Message) (Pawn|GetControlledPawn)))
    (bind _returnvalue_2 (UserInterface|CreateWidget "/Game/UI/WBP_DeathBlowInput.WBP_DeathBlowInput_C" self (Variables|/Script/LeiCS.LeiActionComponent|GetOpponent _returnvalue)))
    (bind _output_get (Variables|Default|SetDeathblowWidget _returnvalue_2))
    (UserInterface|Viewport|AddtoViewport _output_get 0)))