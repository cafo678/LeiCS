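; Player combat character Blueprint that extends parent action, damage, parry and opponent events with tag-driven reactions.
; Deathblow events toggle controller yaw rotation, and the opponent's zero poise strips movement tags, waiting for any directional action to stop.
; Hits remove input tags and play montages chosen by defense state, staggering at zero poise; parries drive a timeline knockback.
; Debug-style key bindings make the AI character kick.
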(event EventOnOpponentActionStarted
  (params (Opponent :type Actor%20Object%20Reference) (ActionTagID :type Gameplay%20Tag%20Structure) (ActionDirectionTag :type Gameplay%20Tag%20Structure) (bIsDirectional :type Boolean))
  (|CallParentFunction Opponent ActionTagID ActionDirectionTag bIsDirectional)
  (Delegates|OnOpponentActionStartedBP ActionTagID ActionDirectionTag))

(event EventOnParryReceived
  (params (BacklashDeltaLocation :type Float%20%28single-precision%29) (BacklashDuration :type Float%20%28single-precision%29))
  (|CallParentFunction BacklashDeltaLocation BacklashDuration)
  (|OnParryReceivedBP BacklashDeltaLocation BacklashDuration))

(event EventOnOpponentActionStopped
  (params (Opponent :type Actor%20Object%20Reference) (ActionTagID :type Gameplay%20Tag%20Structure) (ActionDirectionTag :type Gameplay%20Tag%20Structure) (bIsDirectional :type Boolean))
  (|CallParentFunction Opponent ActionTagID ActionDirectionTag bIsDirectional)
  (Delegates|OnOpponentActionStoppedBP ActionTagID))

(event EventOnDamageReceived
  (params (Delta :type Float%20%28single-precision%29) (InInstigator :type Actor%20Object%20Reference) (InstigatorActionTagID :type Gameplay%20Tag%20Structure))
  (|CallParentFunction Delta InInstigator InstigatorActionTagID)
  (|OnDamageReceivedBP Delta InInstigator InstigatorActionTagID))

(event EventOnActionStarted
  (params (Character :type Actor%20Object%20Reference) (ActionTagID :type Gameplay%20Tag%20Structure) (ActionDirectionTag :type Gameplay%20Tag%20Structure) (bIsDirectional :type Boolean))
  (|CallParentFunction Character ActionTagID ActionDirectionTag bIsDirectional)
  (Delegates|OnActionStartedBP ActionTagID))

(event EventOnCombatSceneEntered
  (params (Opponent :type Actor%20Object%20Reference))
  (|CallParentFunction Opponent)
  (Delegates|OnCombatSceneEnteredBP Opponent))

(event Input|GamepadEvents|GamepadFaceButtonBottom
  (params (Key :type Key%20Structure :default "None"))
  (:Pressed
    (bind _returnvalue (Actor|GetActorOfClass "/Game/AI/BP_AICharacter.BP_AICharacter_C"))
    (Class|LeiActionComponent|StartActionbyTagID (Variables|/Script/LeiCS.LeiCharacter|GetActionComponent _returnvalue) 0 "(TagName=\"Action.Kick\")")))

(event Input|MouseEvents|LeftMouseButton
  (params (Key :type Key%20Structure :default "None"))
  (:Pressed
    (bind _returnvalue (Actor|GetActorOfClass "/Game/AI/BP_AICharacter.BP_AICharacter_C"))
    (Class|LeiActionComponent|StartActionbyTagID (Variables|/Script/LeiCS.LeiCharacter|GetActionComponent _returnvalue) 0 "(TagName=\"Action.Kick\")")))

(fn ConstructionScript)

(fn OnOpponentActionStartedBP
  (params (ActionTagID :type Gameplay%20Tag%20Structure) (ActionDirectionTag :type Gameplay%20Tag%20Structure))
  (|SwitchGameplayTag ActionTagID
    (:Action.Deathblow
      (OnOpponentAction|OnOpponentDeathblow))))

(fn RemoveTagsonOpponentZeroPoise
  (params (ActionActor :type Actor%20Object%20Reference) (ActionTagID :type Gameplay%20Tag%20Structure) (ActionDirectionTag :type Gameplay%20Tag%20Structure) (bIsDirectional :type Boolean))
  (EventDispatchers|UnbindEventfromOnActionStoppedDelegate (Variables|Default|GetActionComponent) (EventDispatchers|CreateEvent :!event RemoveTagsonOpponentZeroPoise))
  (GameplayTags|RemoveGameplayTag (Variables|/Script/LeiCS.LeiActionComponent|GetActiveGameplayTags (Variables|Default|GetActionComponent)) "(TagName=\"CanMove\")" :!class /Script/GameplayTags.BlueprintGameplayTagLibrary)
  (GameplayTags|RemoveGameplayTag (Variables|/Script/LeiCS.LeiActionComponent|GetActiveGameplayTags (Variables|Default|GetActionComponent)) "(TagName=\"CanProcessDirectionalInput\")" :!class /Script/GameplayTags.BlueprintGameplayTagLibrary))

(fn OnActionStartedBP
  (params (ActionTagID :type Gameplay%20Tag%20Structure))
  (|SwitchGameplayTag ActionTagID
    (:Action.Deathblow
      (OnAction|OnDeathlow))))

(fn OnDeathlow
  (Variables|Default|SetbUseControllerRotationYaw false))

(fn OnOpponentDeathblow
  (Variables|Default|SetbUseControllerRotationYaw false))

(fn OnOpponentActionStoppedBP
  (params (ActionTagID :type Gameplay%20Tag%20Structure))
  (|SwitchGameplayTag ActionTagID
    (:Action.Deathblow
      (OnOpponentActionStopped|OnOpponentDeathblowStopped))))

(fn OnOpponentDeathblowStopped
  (Variables|Default|SetbUseControllerRotationYaw true))

(fn OnCombatSceneEnteredBP
  (params (Opponent :type Actor%20Object%20Reference))
  (bind _returnvalue (Class|LeiActionComponentInterface|GetActionComponent(Message) Opponent))
  (Class|LeiAttributeSet|AddAttributeChangedDelegate (Variables|/Script/LeiCS.LeiActionComponent|GetAttributeSet _returnvalue) "(TagName=\"Attribute.Poise\")" (EventDispatchers|CreateEvent :!event OnOpponentPoiseChanged)))

(fn OnOpponentPoiseChanged
  (params (Value :type Float%20%28single-precision%29) (MaxValue :type Float%20%28single-precision%29) (MinValue :type Float%20%28single-precision%29))
  (if (<= Value 0.0)
    (if (== (.actiontagid (Variables|/Script/LeiCS.LeiActionComponent|GetCurrentDirectionalActionDetails (Variables|Default|GetActionComponent))) "(TagName=\"Action.None\")")
      (OnOpponentAttribute|RemoveTagsonOpponentZeroPoise)
      (else
        (EventDispatchers|BindEventtoOnActionStoppedDelegate (Variables|Default|GetActionComponent) (EventDispatchers|CreateEvent :!event RemoveTagsonOpponentZeroPoise))))))