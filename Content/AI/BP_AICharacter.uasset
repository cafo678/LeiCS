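; BP_AICharacter is an AI-controlled combat character that reacts to the player through its behavior tree.
; On entering a combat scene, it runs the BP_AIController's behavior tree and, if that succeeds, focuses on the player and stores them in the blackboard.
; When a player action starts with a valid direction tag, it sets a blackboard flag, passing on only that an action began, not its direction.
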(event EventOnCombatSceneEntered
  (params (PlayerCharacter :type Actor%20Object%20Reference) (CombatSceneEnemies :type Set%20of%20Actor%20Object%20References))
  (Utilities|FlowControl|Sequence
    (:then_0
      (bind _asbp_aicontroller (Utilities|Casting|CastToBP_AIController (Pawn|GetController)))
      (bind _returnvalue (AI|RunBehaviorTree _asbp_aicontroller (Variables|/Script/LeiCS.LeiAIController|GetBehaviorTree _asbp_aicontroller)))
      (if _returnvalue
        (AI|SetFocus _asbp_aicontroller PlayerCharacter)
        (AI|Components|Blackboard|SetValueasObject (AI|GetBlackboard 0) (Utilities|Name|MakeLiteralName "Playerpawn") PlayerCharacter)))))

(event EventOnPlayerActionStarted
  (params (ActionTagID :type Gameplay%20Tag%20Structure) (DirectionTag :type Gameplay%20Tag%20Structure))
  (if (GameplayTags|IsGameplayTagValid DirectionTag)
    (AI|Components|Blackboard|SetValueasBool (AI|GetBlackboard 0) (Utilities|Name|MakeLiteralName "PlayerActionJustStarted") true)))

(fn ConstructionScript)