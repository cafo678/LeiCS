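; Player character Blueprint with Enhanced Input movement and look, plus a one-way switch into a combat stance.
; IA_Move feeds MoveRight and MoveForward and tracks input release, while IA_Look drives controller yaw and pitch.
; Key 1 plays an idle-to-combat montage, whose blend-out sets IsCombat and turns off orient-to-movement and spring arm pawn control rotation.
; Tick is empty and a velocity debug print is left unconnected.
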(event Input|EnhancedActionEvents|EnhancedInputActionIA_Move
  (params (ActionValue :type Vector%202D%20Structure) (ElapsedSeconds :type Float%20%28double-precision%29) (TriggeredSeconds :type Float%20%28double-precision%29) (InputAction :type Input%20Action%20Object%20Reference :default "/Game/Input/IA_Move.IA_Move"))
  ;[1 1 1] Movement
  (:Triggered
    (Class|LeiCharacter|MoveRight (.x ActionValue))
    (Class|LeiCharacter|MoveForward (.y ActionValue))
    (Variables|Default|SetHasUserReleasedMovementInput false))
  (:Completed
    (Variables|Default|SetHasUserReleasedMovementInput true)))

(event Input|EnhancedActionEvents|EnhancedInputActionIA_Look
  (params (ActionValue :type Vector%202D%20Structure) (ElapsedSeconds :type Float%20%28double-precision%29) (TriggeredSeconds :type Float%20%28double-precision%29) (InputAction :type Input%20Action%20Object%20Reference :default "/Game/Input/IA_Look.IA_Look"))
  ;[1 1 1] Camera
  (:Triggered
    (Pawn|Input|AddControllerYawInput (.x ActionValue))
    (Pawn|Input|AddControllerPitchInput (.y ActionValue))))

(event EventTick
  (params (DeltaSeconds :type Float%20%28single-precision%29)))

(event Input|KeyboardEvents|1
  (params (Key :type Key%20Structure :default "None"))
  (:Pressed
    (Animation|Montage|PlayMontage (Variables|Character|GetMesh) "/Game/Sword_Animations/Animations/Sequence/01_Idle/Idle_To_Idle_Combat_Seq_Montage.Idle_To_Idle_Combat_Seq_Montage"
      (:OnBlendOut
        (Variables|Default|SetbIsCombat true)
        (Variables|/Script/Engine.CharacterMovementComponent|SetbOrientRotationToMovement (Variables|Default|GetCharacterMovementComponent) false)
        (Variables|/Script/Engine.SpringArmComponent|SetbUsePawnControlRotation (Variables|Default|GetSpringArmComponent) false)))))

(fn ConstructionScript)