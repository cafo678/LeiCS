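; Ground indicator actor that projects a colored decal for a circular or square area of effect and detects players inside it.
; The construction script sizes the decal from AOEExtent, sets its texture and color through a dynamic material, and sizes either Sphere or Box while zeroing the other, based on CircleAOE.
; IsPlayerInAOE queries the active shape and returns whether a LeiPlayerCharacter overlaps it, along with the first one found.
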(event EventBeginPlay)

(event Collision|EventActorBeginOverlap
  (params (OtherActor :type Actor%20Object%20Reference)))

(event EventTick
  (params (DeltaSeconds :type Float%20%28single-precision%29)))

(fn ConstructionScript
  (bind _aoeextent (Variables|Default|GetAOEExtent))
  (bind _aoeextent_2 (Variables|Default|GetAOEExtent))
  (Class|LeiBlueprintFunctionLibrary|SetDecalSize (Variables|Default|GetDecal) (Math|Vector|MakeVector 1e+01 (.y _aoeextent) (.z _aoeextent)))
  (if (Variables|Default|GetCircleAOE)
    (Components|Sphere|SetSphereRadius (Variables|Default|GetSphere) (* (.y (Variables|Default|GetAOEExtent)) 0.71) true)
    (Components|Box|SetBoxExtent (Variables|Default|GetBox) "0, 0, 0" true)
    (bind _returnvalue (Rendering|Material|CreateDynamicMaterialInstance (Variables|Default|GetDecal) :!class /Script/Engine.DecalComponent))
    (Rendering|Material|SetTextureParameterValue _returnvalue "Texture" "/Game/Textures/AoE/CircleAoE.CircleAoE")
    (Rendering|Material|SetVectorParameterValue _returnvalue "Color" (Variables|Default|GetAOEColor) :!class /Script/Engine.MaterialInstanceDynamic)
    (else
      (Components|Box|SetBoxExtent (Variables|Default|GetBox) (Math|Vector|MakeVector 5e+01 (.y _aoeextent_2) (.z _aoeextent_2)) true)
      (Components|Sphere|SetSphereRadius (Variables|Default|GetSphere) 0.0 true)
      (bind _returnvalue_2 (Rendering|Material|CreateDynamicMaterialInstance (Variables|Default|GetDecal) :!class /Script/Engine.DecalComponent))
      (Rendering|Material|SetTextureParameterValue _returnvalue_2 "Texture" "/Game/Textures/AoE/SquareAoE.SquareAoE")
      (Rendering|Material|SetVectorParameterValue _returnvalue_2 "Color" (Variables|Default|GetAOEColor) :!class /Script/Engine.MaterialInstanceDynamic))))

(fn IsPlayerinAOE
  (if (Variables|Default|GetCircleAOE)
    (LocalVariables|SetPlayer (Utilities|Array|Get(acopy) (Collision|GetOverlappingActors (Variables|Default|GetSphere) "/Script/LeiCS.LeiPlayerCharacter" :!class /Script/Engine.PrimitiveComponent)))
    (else
      (LocalVariables|SetPlayer (Utilities|Array|Get(acopy) (Collision|GetOverlappingActors (Variables|Default|GetBox) "/Script/LeiCS.LeiPlayerCharacter" :!class /Script/Engine.PrimitiveComponent)))))
  (bind _player (LocalVariables|GetPlayer)
    (:then
      (return true _player))
    (:else
      (return false 0))))